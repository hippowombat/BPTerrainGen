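; Editor terrain generator actor that builds a Landscape heightmap from procedural Perlin and Voronoi noise.
; The construction script creates a dynamic instance of MI_TerrainConstructor from its noise and height variables, then redraws when HotCookLandscape is set.
; DrawToRT renders that material to a render target and imports it into the Landscape as a heightmap.
; RandomizeTerrainLocation offsets the world-aligned noise randomly and rebuilds the terrain.
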(event `DrawToRT`
  ;[1 1 1] Update Heightmap Render Target, apply Heightmap RT to Landscape, updating geometry/collisions
  (`KismetRenderingLibrary.DrawMaterialToRenderTarget` (`self.RT`) (`self.TerrainMat`))
  (`LandscapeProxy.LandscapeImportHeightmapFromRenderTarget` (`self.Landscape`) (`self.RT`)))

(event `RandomizeTerrainLocation`
  ;[1 1 1] Apply random location offset to world-aligned noise textures generated for heightmap, updates landscape when called
  (set `self.RandomOffset` (`KismetMathLibrary.RandomFloatInRange` -5000000.0 5000000.0))
  (`MaterialInstanceDynamic.SetScalarParameterValue` (`self.TerrainMat`) "RandomOffset" (`self.RandomOffset`))
  (`self.DrawToRT`))

(fn `Assign Variables to Terrain Construction Dynamic Material`
  (bind _returnvalue (`KismetMaterialLibrary.CreateDynamicMaterialInstance` "/Game/TerrainEditor/Materials/Instances/MI_TerrainConstructor.MI_TerrainConstructor"))
  (bind _output_get (set `self.TerrainMat` _returnvalue))
  (`MaterialInstanceDynamic.SetScalarParameterValue` _output_get "PerlinScale" (`self.PerlinScale`))
  (`MaterialInstanceDynamic.SetScalarParameterValue` _output_get "PerlinContrast" (`self.PerlinContrast`))
  (`MaterialInstanceDynamic.SetScalarParameterValue` _output_get "PerlinStrength" (`self.PerlinStrength`))
  (`MaterialInstanceDynamic.SetScalarParameterValue` _output_get "VoronoiContrast" (`self.VoronoiContrast`))
  (`MaterialInstanceDynamic.SetScalarParameterValue` _output_get "VoronoiStrength" (`self.VoronoiStrength`))
  (`MaterialInstanceDynamic.SetScalarParameterValue` _output_get "VoronoiScale" (`self.VoronoiScale`))
  (`MaterialInstanceDynamic.SetScalarParameterValue` _output_get "OverallHeight" (`self.OverallHeight`))
  (return))

(fn `UserConstructionScript`
  (`self.Assign Variables to Terrain Construction Dynamic Material`)
  (if (`self.HotCookLandscape`)
    (`self.DrawToRT`)))